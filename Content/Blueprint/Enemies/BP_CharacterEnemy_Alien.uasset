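; Alien melee enemy character that reacts to damage, attacks the player and may drop a weapon-type item on death.
; Damage feeds a health component, which spawns damage numbers and randomly triggers confusion stuns, hit animations or timed slowdowns interpolated on Tick.
; Light and heavy attack montages use notifies to fire sphere traces that damage Player-tagged actors, while toggling move and attack flags.
; Death unpossesses, triggers the drop, then ragdolls after its montage.
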(event OnHealthChange(OnePsychoHealth)
  (params (Health :type Float%20%28single-precision%29) (Damage :type Float%20%28single-precision%29))
  (if (not (Variables|Flags|GetbIsDead))
    (if (> (Math|Random|RandomFloat) (Variables|Chance|GetConfusionChance))
      (CallFunction|ConfusionEnabledTimer)
      (else
        (CallFunction|HitAnim)))
    (bind _returnvalue (Game|SpawnActorfromClass "/Game/Blueprint/InteractEnvir/DisplayDamage/DisplayDamageActor.DisplayDamageActor_C" (Math|Transform|MakeTransform (+ (+ (Math|Vector|MakeVector (Math|Random|RandomFloatinRange -2e+01 2e+01) (Math|Random|RandomFloatinRange -2e+01 2e+01) 0.0) (Variables|Default|GetSpawnOffsetLocalDamage)) (Transformation|GetActorLocation))) "AlwaysSpawn" 0 0))
    (Default|InitActor _returnvalue Damage Health)
    (if (> (Math|Random|RandomFloat) (Variables|Chance|GetSlowDownSpeedChance))
      (Variables|Flags|SetSlowDownSpeed true)
      (Utilities|Time|SetTimerbyEvent (delegate Custom|SlowDownDisabled) 2.0))))

(event OnDead(OnePsychoHealth)
  (bind _deadsanim (Variables|Default|GetDeadsAnim))
  (bind _mesh (Variables|Character|GetMesh))
  (bind _returnvalue (Utilities|Array|Length _deadsanim))
  (bind _returnvalue_2 (- _returnvalue 1))
  (bind _output (Utilities|Array|Get(acopy) _deadsanim _returnvalue_2))
  (if (not (Variables|Flags|GetbIsDead))
    (CallFunction|DeadEvent)
    (Utilities|IsValid _output
      (:Is%20Valid
        (Animation|Montage|PlayMontage _mesh _output
          (:OnCompleted
            (Collision|SetCollisionEnabled _mesh "PhysicsOnly")
            (Collision|SetCollisionResponsetoChannel (Variables|Collision|GetCapsuleComponent) "ECC_Pawn" "ECR_Ignore")
            (Collision|SetCollisionProfileName _mesh "PhysicsActor" true :!class /Script/Engine.PrimitiveComponent)
            (Physics|SetSimulatePhysics _mesh true)))))))

(event Custom|SlowDownDisabled
  (Variables|Flags|SetSlowDownSpeed false))

(event EventBeginPlay
  (CallFunction|InitDropComponent))

(event EventMeleeAtackHeavy
  (bind _baseheavydamage (Variables|Combat|GetBaseHeavyDamage))
  (bind _heavyattackanim (Variables|Combat|GetHeavyAttackAnim))
  (CallFunction|SetStateAttack false)
  (CallFunction|SetStateMovement false)
  (bind _notifyname (Animation|Montage|PlayMontage (Variables|Character|GetMesh) (Utilities|Array|Get(acopy) _heavyattackanim (Math|Random|RandomInteger (Utilities|Array|Length _heavyattackanim))))
    (:OnCompleted
      (CallFunction|SetStateMovement true :!label _label)
      (CallFunction|SetStateAttack true))
    (:OnInterrupted
      (goto _label))
    (:OnNotifyBegin
      (if (Utilities|Name|Equal(Name) _notifyname "Attack") ; Heavy
        (Utilities|MeleeTrace 5e+01 1.3e+02 (Math|Random|RandomFloatinRange (- _baseheavydamage 1e+01) (+ _baseheavydamage 5e+01)) (Variables|Combat|GetHeavyRadius))))))

(event EventTick
  (params (DeltaSeconds :type Float%20%28single-precision%29))
  (Variables|Default|SetDeltaTime DeltaSeconds)
  (Utilities|ChangeSpeddbyHit))

(event Game|Damage|EventAnyDamage
  (params (Damage :type Float%20%28single-precision%29) (DamageType :type Damage%20Type%20Object%20Reference) (InstigatedBy :type Controller%20Object%20Reference) (DamageCauser :type Actor%20Object%20Reference))
  (Class|OnePsychoHealthComponent|ChangeHealthValue (Variables|Default|GetOnePsychoHealth) (* Damage -1.0)))

(event EventMeleeAtackLight
  (bind _baselightdamage (Variables|Combat|GetBaseLightDamage))
  (bind _lightattackanim (Variables|Combat|GetLightAttackAnim))
  (CallFunction|SetStateAttack false)
  (CallFunction|SetStateMovement false)
  (bind _notifyname (Animation|Montage|PlayMontage (Variables|Character|GetMesh) (Utilities|Array|Get(acopy) _lightattackanim (Math|Random|RandomInteger (Utilities|Array|Length _lightattackanim))))
    (:OnCompleted
      (CallFunction|SetStateMovement true :!label _label)
      (CallFunction|SetStateAttack true))
    (:OnInterrupted
      (goto _label))
    (:OnNotifyBegin
      (if (Utilities|Name|Equal(Name) _notifyname "Attack") ; Light
        (Utilities|MeleeTrace 5e+01 1.5e+02 (Math|Random|RandomFloatinRange (- _baselightdamage 1e+01) (+ _baselightdamage 2e+01)) (Variables|Combat|GetLightRadius))))))

(fn ConstructionScript)

(fn SetStateMovement
  (params (CanMove :type Boolean))
  (Variables|Flags|SetCanMove CanMove))

(fn SetStateAttack
  (params (CanAttack :type Boolean))
  (Variables|Flags|SetCanAttack CanAttack))

(fn DeadEvent
  (bind _dropcomponent (Variables|Default|GetDropComponent))
  (Pawn|UnPossess (Pawn|GetController))
  (Actor|SetLifeSpan 5.0)
  (CallFunction|SetStateMovement false)
  (CallFunction|SetStateAttack false)
  (Variables|Flags|SetbIsDead true)
  (Utilities|IsValid _dropcomponent
    (:Is%20Valid
      (Default|Drop _dropcomponent))))

(fn InitDropComponent
  (bind _returnvalue (Math|Random|RandomIntegerinRange 0 3))
  (bind _returnvalue_2 (Utilities|Select :Index _returnvalue :Option%200 "RifleType" :Option%201 "ShotGunType" :Option%202 "SniperRifleType" :Option%203 "LauncherType"))
  (if (> (Math|Random|RandomFloat) (Variables|Chance|GetDropChance))
    (bind _returnvalue_3 (AddComponent|AddBPDropItemComponent))
    (Variables|Default|SetDropComponent _returnvalue_3)
    (Variables|/Game/Blueprint/Components/BP_DropItemComponent.BP_DropItemComponent_C|SetType _returnvalue_3 _returnvalue_2)
    (Utilities|FlowControl|Sequence
      (:then_0
        (switch Utilities|FlowControl|Switch|SwitchonEWeaponType _returnvalue_2
          (:RifleType
            (LocalVariables|SetCout 15))
          (:ShotGunType
            (LocalVariables|SetCout 6))
          (:SniperRifleType
            (LocalVariables|SetCout 3))
          (:LauncherType
            (LocalVariables|SetCout 2))))
      (:then_1
        (Variables|/Game/Blueprint/Components/BP_DropItemComponent.BP_DropItemComponent_C|SetCout _returnvalue_3 (LocalVariables|GetCout))))))

(fn ConfusionEnabledTimer
  (bind _confusionanim (Variables|Default|GetConfusionAnim))
  (CallFunction|SetStateMovement false)
  (bind _output_get (Variables|Default|SetCurrentMontage (Utilities|Array|Get(acopy) _confusionanim (Math|Random|RandomIntegerinRange 0 (- (Utilities|Array|Length _confusionanim) 1)))))
  (bind _returnvalue (Animation|GetPlayLength _output_get))
  (Utilities|Time|SetTimerbyFunctionName 0 "ConfusionDisabledTimer" _returnvalue)
  (Animation|PlayAnimMontage (Variables|Default|GetCurrentMontage) 1.0 "None")
  (Variables|/Script/Engine.CharacterMovementComponent|SetMaxWalkSpeed (Variables|Character|GetCharacterMovement) 0.0)
  (Variables|Flags|SetbIsConfused true))

(fn ConfusionDisabledTimer
  (CallFunction|SetStateMovement true)
  (Variables|/Script/Engine.CharacterMovementComponent|SetMaxWalkSpeed (Variables|Character|GetCharacterMovement) 4e+02))

(fn HitAnim
  (if (not (Variables|Flags|GetbIsConfused))
    (if (> (Math|Random|RandomFloat) (Variables|Chance|GetHitAnimChance))
      (Animation|PlayAnimMontage "/Game/Blueprint/Enemies/AlienSoldier/Anim/Hit_To_Body_mixamo_com_Montage.Hit_To_Body_mixamo_com_Montage" 1.0 "None"))))

(fn ICanAttack
  (return (Variables|Flags|GetCanAttack)))

(fn ICanMove
  (return (Variables|Flags|GetCanMove)))