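; Boss-mounted grenade launcher that automatically fires explosive missiles on a looping timer while its boss owner is alive.
; Each tick of the timer reads the owning boss's health, then plays the Shoot timeline or clears the timer once health is depleted.
; The timeline's Shoot event spawns a missile just ahead of the Arrow and configures its mesh, effects, speed and radial damage through InitProjectile.
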(event Custom|FireRocketLauncher
  (bind _returnvalue (Components|GetOwner))
  (bind _arrow (Variables|Default|GetArrow))
  (bind _asbp_character_enemy_boss (Utilities|Casting|CastToBP_CharacterEnemy_Boss _returnvalue))
  (bind _returnvalue_2 (Class|OnePsychoHealthComponent|GetCurrentHealth (Variables|/Game/Blueprint/Enemies/BP_CharacterEnemy_Alien.BP_CharacterEnemy_Alien_C|GetOnePsychoHealth _asbp_character_enemy_boss)))
  (if (> _returnvalue_2 0.0)
    (Timeline|Shoot PlayFromStart
      (:Shoot
        (bind _returnvalue_3 (Game|SpawnActorfromClass "/Game/Blueprint/Enemies/Boss/BossGrenadeLauncher/BP_MissleBossGrenadeLauncher.BP_MissleBossGrenadeLauncher_C" (Math|Transform|MakeTransform (+ (* (Math|Vector|GetForwardVector _arrow) 25.0) (Transformation|GetWorldLocation _arrow)) (Transformation|GetWorldRotation _arrow)) "AlwaysSpawn" _returnvalue 0))
        (Class|ProjectileDefault|InitProjectile _returnvalue_3 (Utilities|Struct|MakeProjectileInfo "/Game/Blueprint/Enemies/Boss/BossGrenadeLauncher/BP_MissleBossGrenadeLauncher.BP_MissleBossGrenadeLauncher_C" "/Game/Items/BossMissle/MissleStaticMesh.MissleStaticMesh" (Math|Transform|MakeTransform "0, 0, 0" "90.000000, 0,0.000000" "10.000000,10.000000,10.000000") "/Game/Items/GameActor/Weapons/FX/P_RocketLauncher_Trail_01.P_RocketLauncher_Trail_01" (Math|Transform|MakeTransform "-35.000000,0.000000, 0") 1.0 2e+01 5e+02 1e+03 "SurfaceType_Default" 0 "SurfaceType_Default" 0 "/Game/Items/GameActor/Weapons/FX/P_Grenade_Explosion_01.P_Grenade_Explosion_01" "/Game/Items/GameActor/Weapons/Sound/RocketLauncher/RocketLauncher_Explosion_Cue.RocketLauncher_Explosion_Cue" 3.0 1.5e+02 3e+02 3e+01 2.0))))
    (else
      (Utilities|Time|ClearandInvalidateTimerbyHandle (Variables|Default|GetFireRocketHandleTimer)))))

(event EventBeginPlay
  (bind _returnvalue (Utilities|Time|SetTimerbyEvent (delegate Custom|FireRocketLauncher) 7.0 true))
  (Variables|Default|SetFireRocketHandleTimer _returnvalue))

(event Collision|EventActorBeginOverlap
  (params (OtherActor :type Actor%20Object%20Reference)))

(event EventTick
  (params (DeltaSeconds :type Float%20%28single-precision%29)))

(fn ConstructionScript)