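; Enemy AI controller that runs BT_AI_Base and turns perception of Player-tagged actors into blackboard state.
; On BeginPlay it starts the tree and sets an initial ChaseState.
; Hearing stores the player's location as LastTargetVector and flags CanHearTarget, while other senses set or clear TargetActor, TargetVector and CanSeeTarget.
; Losing sight also zeroes LastTargetVector and draws debug markers at the loss point.
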(event OnTargetPerceptionUpdated(AIPerception)
  (params (Actor :type Actor%20Object%20Reference) (Stimulus :type AI%20Stimulus%20Structure))
  (bind _returnvalue (AI|GetBlackboard 0))
  (bind _returnvalue_2 (AI|GetBlackboard 0))
  (bind _returnvalue_3 (AI|GetBlackboard 0))
  (Utilities|IsValid Actor
    (:Is%20Valid
      (Variables|Default|SetCurrentTarget Actor)
      (if (Actor|ActorHasTag Actor "Player")
        (bind _returnvalue_4 (Class|AIPerceptionSystem|GetSenseClassforStimulus Stimulus))
        (if (== _returnvalue_4 "/Script/AIModule.AISense_Hearing")
          (AI|Components|Blackboard|SetValueasVector _returnvalue (Utilities|Name|MakeLiteralName "LastTargetVector") (Transformation|GetActorLocation (Variables|Default|GetCurrentTarget)))
          (AI|Components|Blackboard|SetValueasBool _returnvalue (Utilities|Name|MakeLiteralName "CanHearTarget") true)
          (elif (.bSuccessfullySensed (Utilities|Struct|BreakAIStimulus Stimulus))
            (AI|Components|Blackboard|SetValueasObject _returnvalue_2 (Utilities|Name|MakeLiteralName "TargetActor") (Variables|Default|GetCurrentTarget))
            (AI|Components|Blackboard|SetValueasVector _returnvalue_2 (Utilities|Name|MakeLiteralName "TargetVector") (Transformation|GetActorLocation (Variables|Default|GetCurrentTarget)))
            (AI|Components|Blackboard|SetValueasBool _returnvalue_2 (Utilities|Name|MakeLiteralName "CanSeeTarget") true)
            (else
              (Utilities|IsValid (Variables|Default|GetCurrentTarget)
                (:Is%20Valid
                  (AI|Components|Blackboard|SetValueasObject _returnvalue_3 (Utilities|Name|MakeLiteralName "TargetActor") 0)
                  (AI|Components|Blackboard|SetValueasVector _returnvalue_3 (Utilities|Name|MakeLiteralName "TargetVector") "0, 0, 0")
                  (AI|Components|Blackboard|SetValueasBool _returnvalue_3 (Utilities|Name|MakeLiteralName "CanSeeTarget") false)
                  (AI|Components|Blackboard|SetValueasVector _returnvalue_3 (Utilities|Name|MakeLiteralName "LastTargetVector") "0, 0, 0")
                  (Rendering|Debug|DrawDebugSphere (Transformation|GetActorLocation (Variables|Default|GetCurrentTarget)) 12.0 12 "(R=0.000000,G=0.623529,B=1.000000,A=1.000000)" 1e+01)
                  (Rendering|Debug|DrawDebugString (Transformation|GetActorLocation (Variables|Default|GetCurrentTarget)) "I've lost target here" 0 "(R=0.000000,G=0.000000,B=0.000000,A=1.000000)" 1e+01))
                (:Is%20Not%20Valid
                  (Development|PrintString "TargetPerseption: Target isn't valid"))))))))
    (:Is%20Not%20Valid
      (Variables|Default|SetCurrentTarget 0))))

(event EventBeginPlay
  (AI|RunBehaviorTree "/Game/Blueprint/Enemies/Common/BT_AI_Base.BT_AI_Base")
  (AI|Components|Blackboard|SetValueasEnum (AI|GetBlackboard 0) (Utilities|Name|MakeLiteralName "ChaseState") 3))

(fn ConstructionScript)