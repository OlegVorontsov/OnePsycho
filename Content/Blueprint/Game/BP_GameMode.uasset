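; Game mode that spawns and respawns the player at phase-named player starts.
; ChoosePlayerStart always picks the Phase1 start.
; TryToRespawn asks BP_GameState whether respawning is allowed, maps the returned current phase to its matching start name and restarts player controller 0 there, returning whether it succeeded.
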(event EventBeginPlay)

(event EventTick
  (params (DeltaSeconds :type Float%20%28single-precision%29)))

(fn ConstructionScript)

(fn TrytoRespawn
  (bind _asbp_game_state (Utilities|Casting|CastToBP_GameState (Game|GetGameState)))
  (bind (_success _currentphase) (Default|CanPlayerRespawn _asbp_game_state))
  (if _success
    (Class|GameModeBase|RestartPlayeratPlayerStart (Game|GetPlayerController 0) (Class|GameModeBase|FindPlayerStart 0 (Utilities|Select :Index _currentphase :NewEnumerator0 "Phase1" :NewEnumerator1 "Phase2" :NewEnumerator2 "Phase3" :NewEnumerator3 "Phase4" :NewEnumerator4 "Phase5")))
    (return true)
    (else
      (return _success))))

(fn ChoosePlayerStart
  (params (Player :type Controller%20Object%20Reference))
  (return (Class|GameModeBase|FindPlayerStart Player "Phase1")))