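; An invulnerability power-up pickup actor, a child of a pickup base that handles overlap with characters.
; On a character overlap it casts the inventory's owner to BP_Character, enables invulnerability on it and reports the pickup as successful.
; While in the level it spins by adding a fixed local rotation every tick, not scaled by delta time.
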(event EventBeginPlay
  (|CallParentFunction) ; This node is disabled and will not be called.\nDrag off pins to build functionality.
)

(event Collision|EventActorBeginOverlap
  (params (OtherActor :type Actor%20Object%20Reference))
  (|CallParentFunction OtherActor) ; This node is disabled and will not be called.\nDrag off pins to build functionality.
)

(event EventTick
  (params (DeltaSeconds :type Float%20%28single-precision%29))
  (|CallParentFunction DeltaSeconds)
  (Transformation|AddActorLocalRotation "0.000000,0.000000,1.500000" false false))

(event EventOverlapCharacter
  (params (ToInventory :type Character%20Inventory%20Component%20Object%20Reference))
  (|CallParentFunction ToInventory)
  (bind _asbp_character (Utilities|Casting|CastToBP_Character (Components|GetOwner ToInventory)))
  (Class|OnePsychoCharacter|InvulnerabilityEnabled _asbp_character)
  (CallFunction|PickUpSuccess))

(fn ConstructionScript
  (|CallParentFunction))