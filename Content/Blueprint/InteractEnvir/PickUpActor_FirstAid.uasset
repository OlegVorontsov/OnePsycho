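; First-aid pickup actor that restores health to the player character on overlap.
; It extends the parent pickup's OverlapCharacter event, casting the inventory component's owner to BP_Character.
; If current health is below 100, it applies Value through CharHealthComponent and calls PickUpSuccess; at full health the pickup is not consumed.
; Tick adds a small local yaw or roll rotation each frame so the item spins, independent of frame time.
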(event EventBeginPlay
  (|CallParentFunction) ; This node is disabled and will not be called.\nDrag off pins to build functionality.
)

(event Collision|EventActorBeginOverlap
  (params (OtherActor :type Actor%20Object%20Reference))
  (|CallParentFunction OtherActor) ; This node is disabled and will not be called.\nDrag off pins to build functionality.
)

(event EventTick
  (params (DeltaSeconds :type Float%20%28single-precision%29))
  (|CallParentFunction DeltaSeconds)
  (Transformation|AddActorLocalRotation "0.000000,1.500000,0.000000" false false))

(event EventOverlapCharacter
  (params (ToInventory :type Character%20Inventory%20Component%20Object%20Reference))
  (|CallParentFunction ToInventory)
  (bind _asbp_character (Utilities|Casting|CastToBP_Character (Components|GetOwner ToInventory)))
  (bind _returnvalue (Class|OnePsychoHealthComponent|GetCurrentHealth (Variables|/Script/OnePsycho.OnePsychoCharacter|GetCharHealthComponent _asbp_character)))
  (if (< _returnvalue 1e+02)
    (Class|OnePsychoHealthComponent|ChangeHealthValue (Variables|/Script/OnePsycho.OnePsychoCharacter|GetCharHealthComponent _asbp_character) (Variables|Default|GetValue))
    (CallFunction|PickUpSuccess)))

(fn ConstructionScript
  (|CallParentFunction))