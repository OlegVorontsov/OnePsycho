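; Top-down player character that relays weapon events to its anim instance and HUD, and on death asks the GameMode to respawn or shows the end screen.
; Inventory loads from PlayerState and saves on unpossess; weapons are picked up by timed key hold and dropped as pickup actors.
; Health component events drive blood, invulnerability and shield surface effects.
; The camera boom zooms in timer steps and drifts toward the cursor while moving in aim states.
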(event OnHealthChange(CharHealthComponent)
  (params (Health :type Float%20%28single-precision%29) (Damage :type Float%20%28single-precision%29))
  (bind _returnvalue (Math|Float|MapRangeClamped Health 5e+01 1e+02 1.0 0.0))
  (bind _mesh (Variables|Character|GetMesh))
  (bind _returnvalue_2 (Rendering|Material|GetMaterial _mesh 0))
  (Utilities|FlowControl|Sequence
    (:then_0
      (if (< Damage 0.0)
        (if (> (Math|Random|RandomFloat) 0.6)
          (Rendering|Decal|SpawnDecalatLocation (Utilities|Select :Index (Math|Random|RandomIntegerinRange 0 2) :Option%200 "/Game/Fx_Effect/MS_Blood/Decal/010_Blood_Stain_sgfjdepc/010_Blood_Stain_sgfjdepc_8K_inst.010_Blood_Stain_sgfjdepc_8K_inst" :Option%201 "/Game/Fx_Effect/MS_Blood/Decal/13_Blood_Stain_sheadaac/13_Blood_Stain_sheadaac_8K_inst.13_Blood_Stain_sheadaac_8K_inst" :Option%202 "/Game/Fx_Effect/MS_Blood/Decal/15_Blood_Stain_sg3bbd2c/15_Blood_Stain_sg3bbd2c_8K_inst.15_Blood_Stain_sg3bbd2c_8K_inst") "60.000000,60.000000,60.000000" (+ (Transformation|GetActorLocation) (Math|Vector|MakeVector (Math|Random|RandomFloatinRange -32.0 32.0) (Math|Random|RandomFloatinRange -32.0 32.0) -1e+02)) "-90.000000,0.000000,0.000000" 1e+01))))
    (:then_1
      (bind _asmaterial_instance_dynamic (Utilities|Casting|CastToMaterialInstanceDynamic _returnvalue_2)
        (:then
          (Rendering|Material|SetScalarParameterValue _asmaterial_instance_dynamic "Blood" _returnvalue :!class /Script/Engine.MaterialInstanceDynamic))
        (:CastFailed
          (bind _returnvalue_3 (Rendering|Material|CreateDynamicMaterialInstance _mesh 0 _returnvalue_2 "BloodDynamic" :!class /Script/Engine.PrimitiveComponent))
          (Rendering|Material|SetScalarParameterValue _returnvalue_3 "Blood" _returnvalue :!class /Script/Engine.MaterialInstanceDynamic)
          (Rendering|Material|SetMaterial _mesh 0 _returnvalue_3))))))

(event OnInvulnerabilityChange(CharHealthComponent)
  (params (bIsInvulnerable :type Boolean))
  (bind _mesh (Variables|Character|GetMesh))
  (if bIsInvulnerable
    (bind _returnvalue (UserInterface|CreateWidget "/Game/Blueprint/Widget/Health/InvulnerabilityWidget.InvulnerabilityWidget_C"))
    (UserInterface|Viewport|AddtoViewport _returnvalue 0)
    (Rendering|Material|SetMaterial _mesh 0 "/Game/Blueprint/Character/Mannequin/Character/Materials/M_Male_Body_Invulnerability.M_Male_Body_Invulnerability")
    (else
      (Rendering|Material|SetMaterial _mesh 0 "/Game/Blueprint/Character/Mannequin/Character/Materials/M_Male_Body.M_Male_Body"))))

(event OnShieldChange(CharHealthComponent)
  (params (Shield :type Float%20%28single-precision%29) (Damage :type Float%20%28single-precision%29))
  (bind _mesh (Variables|Character|GetMesh))
  (bind _returnvalue (Class|OnePsychoCharHealthComponent|GetCurrentShield (Variables|Default|GetCharHealthComponent)))
  (if (>= _returnvalue 0.1)
    (Class|PrimitiveComponent|SetPhysMaterialOverride _mesh "/Game/Enviroment/PhysicalMaterials/Shield.Shield")
    (else
      (Class|PrimitiveComponent|SetPhysMaterialOverride _mesh "/Game/Enviroment/PhysicalMaterials/Flesh.Flesh"))))

(event OnSwitchWeapon(CharacterInventoryComponent)
  (params (WeaponIdName :type Name :default "None") (WeaponAdditionalInfo :type Additional%20Weapon%20Info%20Structure) (NewCurrentIndexWeapon :type Integer))
  (bind _asbp_player_controller (Utilities|Casting|CastToBP_PlayerController (Pawn|GetController)))
  (Utilities|IsValid (Variables|/Game/Blueprint/Game/BP_PlayerController.BP_PlayerController_C|GetInGameWidget _asbp_player_controller)
    (:Is%20Valid
      (bind _asweapon_slot (Utilities|Casting|CastToWeaponSlot (Class|PanelWidget|GetChildat (Variables|/Game/Blueprint/Widget/Inventory/InventoryStatsWidget.InventoryStatsWidget_C|GetWeaponSlots_1 (Variables|/Game/Blueprint/Widget/InGameWidget.InGameWidget_C|GetInventoryStatsWidget (Variables|/Game/Blueprint/Game/BP_PlayerController.BP_PlayerController_C|GetInGameWidget _asbp_player_controller))) NewCurrentIndexWeapon)))
      (Default|UpdateInfo _asweapon_slot WeaponIdName (Utilities|Struct|BreakAdditionalWeaponInfo WeaponAdditionalInfo)))))

(event Custom|StartSwitchWeapon
  (params (CatchPickupWeapon :type Pick%20Up%20Actor%20Weapon%20Object%20Reference))
  ;[1 1 1] Пикап оружия (старое)
)

(event Custom|EndSwitchWeapon
  ;[1 1 1] Пикап оружия (старое)
  (Variables|Pickup|SetCatchPickupWeapon 0))

(event Custom|CheckPickUpActor
  (bind _interactpickupactor (Variables|Default|GetInteractPickUpActor))
  (bind _overlappingactors (Collision|GetOverlappingActors _interactpickupactor 0 :!class /Script/Engine.PrimitiveComponent))
  (bind _output (Utilities|Array|Get(acopy) _overlappingactors))
  (Utilities|IsValid _output
    (:Is%20Valid
      (bind _aspick_up_actor_weapon (Utilities|Casting|CastToPickUpActor_Weapon _output))
      (Utilities|IsValid (Variables|Pickup|GetPickUpWidget)
        (:Is%20Valid
          (if (not (Utilities|Name|Equal(Name) (Variables|/Game/Blueprint/Widget/Inventory/BPW_PickUpWidget.BPW_PickUpWidget_C|GetIdWeaponName (Variables|Pickup|GetPickUpWidget)) (Variables|/Game/Blueprint/InteractEnvir/PickUpActor_Weapon.PickUpActor_Weapon_C|GetItemName _aspick_up_actor_weapon)))
            (Default|ChangeName (Variables|Pickup|GetPickUpWidget) (Utilities|Text|ToText(Name) (Variables|/Game/Blueprint/InteractEnvir/PickUpActor_Weapon.PickUpActor_Weapon_C|GetItemName _aspick_up_actor_weapon)))))
        (:Is%20Not%20Valid
          (bind _returnvalue (UserInterface|CreateWidget :Class "/Game/Blueprint/Widget/Inventory/BPW_PickUpWidget.BPW_PickUpWidget_C" :IdWeaponName (Variables|/Game/Blueprint/InteractEnvir/PickUpActor_Weapon.PickUpActor_Weapon_C|GetItemName _aspick_up_actor_weapon)))
          (UserInterface|Viewport|AddtoViewport _returnvalue 0)
          (Variables|Pickup|SetPickUpWidget _returnvalue))))
    (:Is%20Not%20Valid
      (Utilities|IsValid (Variables|Pickup|GetPickUpWidget)
        (:Is%20Valid
          (Widget|RemovefromParent (Variables|Pickup|GetPickUpWidget))
          (Variables|Pickup|SetPickUpWidget 0))))))

(event EventTick
  (params (DeltaSeconds :type Float%20%28single-precision%29))
  (CallFunction|CameraSlidetoCursorV2 DeltaSeconds))

(event EventWeaponFireStartBP
  (params (Anim :type Anim%20Montage%20Object%20Reference))
  (Default|Fire (Variables|Default|GetMannequinAnimInstance) Anim))

(event EventWeaponReloadStartBP
  (params (Anim :type Anim%20Montage%20Object%20Reference))
  (Default|Reload (Variables|Default|GetMannequinAnimInstance) Anim)
  (bind _asbp_player_controller (Utilities|Casting|CastToBP_PlayerController (Pawn|GetController)))
  (Utilities|IsValid (Variables|/Game/Blueprint/Game/BP_PlayerController.BP_PlayerController_C|GetInGameWidget _asbp_player_controller)
    (:Is%20Valid
      (Default|WeaponReloadStart (Variables|/Game/Blueprint/Widget/InGameWidget.InGameWidget_C|GetInventoryStatsWidget (Variables|/Game/Blueprint/Game/BP_PlayerController.BP_PlayerController_C|GetInGameWidget _asbp_player_controller)) (Class|OnePsychoCharacter|GetCurrentWeaponIndex)))))

(event EventWeaponReloadEndBP
  (params (bIsSuccess :type Boolean))
  (Default|ReloadEnd (Variables|Default|GetMannequinAnimInstance) bIsSuccess)
  (bind _asbp_player_controller (Utilities|Casting|CastToBP_PlayerController (Pawn|GetController)))
  (Utilities|IsValid (Variables|/Game/Blueprint/Game/BP_PlayerController.BP_PlayerController_C|GetInGameWidget _asbp_player_controller)
    (:Is%20Valid
      (Default|WeaponReloadEnd (Variables|/Game/Blueprint/Widget/InGameWidget.InGameWidget_C|GetInventoryStatsWidget (Variables|/Game/Blueprint/Game/BP_PlayerController.BP_PlayerController_C|GetInGameWidget _asbp_player_controller)) (Class|OnePsychoCharacter|GetCurrentWeaponIndex) bIsSuccess))))

(event EventDropWeapontoWorld
  (params (DropItemInfo :type Drop%20Item%20Structure))
  (|CallParentFunction DropItemInfo)
  (CallFunction|DropItem DropItemInfo))

(event EventCharDeadBP
  (Collision|SetCollisionResponsetoChannel (Variables|Default|GetCapsuleComponent) "ECC_Pawn" "ECR_Ignore")
  (Actor|SetLifeSpan (Class|OnePsychoCharacter|GetCurrentWeapon) 2e+01)
  (Actor|SetLifeSpan 2e+01)
  (bind _asbp_game_mode (Utilities|Casting|CastToBP_GameMode (Game|GetGameMode)))
  (bind _success (Default|TrytoRespawn _asbp_game_mode))
  (if (not _success)
    (bind _returnvalue (UserInterface|CreateWidget "/Game/Blueprint/Widget/BPW_EndGameWidget.BPW_EndGameWidget_C"))
    (UserInterface|Viewport|AddtoViewport _returnvalue 0)
    (Variables|/Script/Engine.PlayerController|SetbShowMouseCursor (Game|GetPlayerController 0) true)))

(event EventBeginPlay
  (bind _returnvalue (Game|GetPlayerController 0))
  (bind _asthird_person_anim_bp (Utilities|Casting|CastToThirdPerson_AnimBP (Components|SkeletalMesh|GetAnimInstance (Variables|Character|GetMesh))))
  (Variables|Default|SetMannequinAnimInstance _asthird_person_anim_bp)
  (bind _asbp_player_state (Utilities|Casting|CastToBP_PlayerState (Variables|/Script/Engine.Controller|GetPlayerState _returnvalue)))
  (Class|CharacterInventoryComponent|InitInventory (Variables|Default|GetCharacterInventoryComponent) (Variables|/Game/Blueprint/Game/BP_PlayerState.BP_PlayerState_C|GetWeaponSlots _asbp_player_state) (Variables|/Game/Blueprint/Game/BP_PlayerState.BP_PlayerState_C|GetAmmoSlots _asbp_player_state))
  (bind _asbp_player_controller (Utilities|Casting|CastToBP_PlayerController _returnvalue))
  (Default|InitInventoryStatsWidget (Variables|/Game/Blueprint/Widget/InGameWidget.InGameWidget_C|GetInventoryStatsWidget (Variables|/Game/Blueprint/Game/BP_PlayerController.BP_PlayerController_C|GetInGameWidget _asbp_player_controller)) self)
  (Utilities|Time|SetTimerbyEvent (delegate Custom|CheckPickUpActor) 0.1 true))

(event EventUnpossessed
  (params (OldController :type Controller%20Object%20Reference))
  (bind _characterinventorycomponent (Variables|Default|GetCharacterInventoryComponent))
  (bind _asbp_player_state (Utilities|Casting|CastToBP_PlayerState (Variables|/Script/Engine.Controller|GetPlayerState OldController)))
  (bind _returnvalue (Class|CharacterInventoryComponent|GetWeaponSlots _characterinventorycomponent))
  (bind _returnvalue_2 (Class|CharacterInventoryComponent|GetAmmoSlots _characterinventorycomponent))
  (Default|SaveCurrentInventory _asbp_player_state _returnvalue _returnvalue_2)
  (bind _asbp_player_controller (Utilities|Casting|CastToBP_PlayerController OldController))
  (Default|UnbindAllEvents (Variables|/Game/Blueprint/Widget/InGameWidget.InGameWidget_C|GetInventoryStatsWidget (Variables|/Game/Blueprint/Game/BP_PlayerController.BP_PlayerController_C|GetInGameWidget _asbp_player_controller)) self))

(event Input|ActionEvents|InputActionMovementModeChangeWalk
  (params (Key :type Key%20Structure :default "None"))
  (:Pressed
    (Variables|Default|SetWalkEnabled true)
    (Class|OnePsychoCharacter|ChangeMovementState :!label _label))
  (:Released
    (Variables|Default|SetWalkEnabled false)
    (goto _label)))

(event Input|ActionEvents|InputActionMovementModeChangeSprint
  (params (Key :type Key%20Structure :default "None"))
  (:Pressed
    (Variables|Default|SetSprintRunEnabled true)
    (Class|OnePsychoCharacter|ChangeMovementState :!label _label))
  (:Released
    (Variables|Default|SetSprintRunEnabled false)
    (goto _label)))

(event Input|ActionEvents|InputActionActionNum1
  (params (Key :type Key%20Structure :default "None"))
  ;[1 1 1] Пикап оружия (старое)
)

(event Input|ActionEvents|InputActionActionNum2
  (params (Key :type Key%20Structure :default "None"))
  ;[1 1 1] Пикап оружия (старое)
)

(event Input|ActionEvents|InputActionActionNum3
  (params (Key :type Key%20Structure :default "None"))
  ;[1 1 1] Пикап оружия (старое)
)

(event Input|ActionEvents|InputActionActionNum4
  (params (Key :type Key%20Structure :default "None"))
  ;[1 1 1] Пикап оружия (старое)
)

(event Input|ActionEvents|InputActionInteractPickUpActor
  (params (Key :type Key%20Structure :default "None"))
  (bind _pickupwidget (Variables|Pickup|GetPickUpWidget))
  (:Pressed
    (Variables|Pickup|SetInteractKeyPressed true)
    (bind _returnvalue (Utilities|Time|SetTimerbyFunctionName 0 "Try Pick Up Actor Pressed" (Variables|Pickup|GetPickUpTime)))
    (bind _output_get (Variables|Pickup|SetPickUpPressedTimer _returnvalue))
    (Utilities|IsValid _pickupwidget
      (:Is%20Valid
        (Variables|/Game/Blueprint/Widget/Inventory/BPW_PickUpWidget.BPW_PickUpWidget_C|SetTimer _pickupwidget _output_get))))
  (:Released
    (Variables|Pickup|SetInteractKeyPressed false)
    (Utilities|Time|ClearandInvalidateTimerbyHandle (Variables|Pickup|GetPickUpPressedTimer))))

(event Input|AxisEvents|InputAxisMouseWheel
  (params (AxisValue :type Float%20%28single-precision%29))
  (CallFunction|CameraSlideSmooth AxisValue))

(event Input|MouseEvents|RightMouseButton
  (params (Key :type Key%20Structure :default "None"))
  (:Pressed
    (Variables|Default|SetAimEnabled true)
    (Class|OnePsychoCharacter|ChangeMovementState :!label _label))
  (:Released
    (Variables|Default|SetAimEnabled false)
    (goto _label)))

(event Input|KeyboardEvents|F
  (params (Key :type Key%20Structure :default "None"))
  (:Pressed
    (CallFunction|CameraShakeEvent)))

(event Input|KeyboardEvents|V
  (params (Key :type Key%20Structure :default "None"))
  (:Pressed
    (Animation|Montage|PlayMontage (Variables|Character|GetMesh) "/Game/Blueprint/Character/Mannequin/Animations/AnimStarterPack/ASP_Fire_Shotgun_Ironsights_Montage.ASP_Fire_Shotgun_Ironsights_Montage")))

(event Input|KeyboardEvents|V
  (params (Key :type Key%20Structure :default "None")))

(fn ConstructionScript
  (bind _cameraboom (Variables|Default|GetCameraBoom))
  (Variables|/Script/Engine.SpringArmComponent|SetTargetArmLength _cameraboom (Variables|Camera|Slide|GetHieghtCameraStart))
  (Transformation|SetRelativeRotation _cameraboom (Variables|Camera|Main|GetRotatorCamera) false false)
  (Variables|/Script/Engine.SpringArmComponent|SetbEnableCameraLag _cameraboom (Variables|Camera|Main|GetEnableCameraLag))
  (Variables|/Script/Engine.SpringArmComponent|SetCameraLagSpeed _cameraboom (Variables|Camera|Main|GetCoefSmooth)))

(fn CameraShakeEvent
  (Camera|PlayWorldCameraShake "/Game/Blueprint/Game/BP_ShakeCamera.BP_ShakeCamera_C" (Transformation|GetWorldLocation (Variables|Default|GetTopDownCameraComponent)) 0.0 2e+01))

(fn CameraSlideSmooth
  (params (Value :type Float%20%28single-precision%29))
  (bind _hieghtcamerachangedistance (Variables|Camera|Slide|GetHieghtCameraChangeDistance))
  (bind _cameraboom (Variables|Default|GetCameraBoom))
  (bind _targetarmlength (Variables|/Script/Engine.SpringArmComponent|GetTargetArmLength _cameraboom))
  (if (Variables|Camera|Slide|GetSlideDone)
    (if (!= Value 0.0)
      (if (< Value 0.0)
        (if (>= (Variables|Camera|Slide|GetfHieghtCameraMax) (+ _targetarmlength _hieghtcamerachangedistance))
          (Variables|Camera|Slide|SetSlideUp true)
          (Variables|Camera|Slide|SetSlideDone false :!label _label)
          (bind _returnvalue (Utilities|Time|SetTimerbyFunctionName 0 "CameraSlideSmoothTick" (Variables|Camera|Slide|GetTimerStep) true))
          (Variables|Camera|Slide|SetSide%20Timer _returnvalue))
        (elif (<= (Variables|Camera|Slide|GetfHieghtCameraMin) (- _targetarmlength _hieghtcamerachangedistance))
          (Variables|Camera|Slide|SetSlideUp false)
          (goto _label))))))

(fn CameraSlideSmoothTick
  (bind _hieghtcamerachangeslidestepdistance (Variables|Camera|SlideSmoothTick|GetHieghtCameraChangeSlideStepDistance))
  (bind _cameraboom (Variables|Default|GetCameraBoom))
  (bind _output_get (Variables|Camera|SlideSmoothTick|SetCurrentSlideDistance (+ (Variables|Camera|SlideSmoothTick|GetCurrentSlideDistance) _hieghtcamerachangeslidestepdistance)))
  (Variables|/Script/Engine.SpringArmComponent|SetTargetArmLength _cameraboom (select (Variables|Camera|Slide|GetSlideUp) (+ (Variables|/Script/Engine.SpringArmComponent|GetTargetArmLength _cameraboom) _hieghtcamerachangeslidestepdistance) (- (Variables|/Script/Engine.SpringArmComponent|GetTargetArmLength _cameraboom) _hieghtcamerachangeslidestepdistance)))
  (if (>= _output_get (Variables|Camera|Slide|GetHieghtCameraChangeDistance))
    (Variables|Camera|SlideSmoothTick|SetCurrentSlideDistance 0.0)
    (Variables|Camera|Slide|SetSlideDone true)
    (Utilities|Time|ClearandInvalidateTimerbyHandle (Variables|Camera|Slide|GetSide%20Timer))))

(fn CameraSlidetoCursorV2
  (params (NewParam :type Float%20%28single-precision%29))
  (bind _capsulecomponent (Variables|Default|GetCapsuleComponent))
  (bind _cameraboom (Variables|Default|GetCameraBoom))
  (bind _cameraboom_2 (Variables|Default|GetCameraBoom))
  (bind _returnvalue (Transformation|GetWorldLocation _capsulecomponent))
  (bind _returnvalue_2 (Transformation|GetWorldLocation _cameraboom_2))
  (bind _returnvalue_3 (Class|OnePsychoCharacter|GetCursortoWorld))
  (Variables|SlideToCursor|SetClampedCameraHeight (Math|Float|MapRangeClamped (Variables|/Script/Engine.SpringArmComponent|GetTargetArmLength (Variables|Default|GetCameraBoom)) (Variables|Camera|Slide|GetfHieghtCameraMin) (Variables|Camera|Slide|GetfHieghtCameraMax) 0.5 1.0))
  (Variables|SlideToCursor|SetDistanceCameraBoomChar (Math|Vector|VectorLengthXY (- _returnvalue (Transformation|GetWorldLocation _returnvalue_3))))
  (if (Variables|Default|GetCharMoving)
    (if (or (Utilities|Enum|Equal(Enum) (Variables|Default|GetMovementState) "Aim_State") (Utilities|Enum|Equal(Enum) (Variables|Default|GetMovementState) "AimWalk_State"))
      (if (> (Variables|SlideToCursor|GetDistanceCameraBoomChar) (* (Variables|SlideToCursor|GetClampedCameraHeight) (Variables|SlideToCursor|GetfMinClampDistanceLogicMouseCursorStart)))
        (if (not (> (Math|Vector2D|Vector2DLength (Math|Conversions|ToVector2D(Vector) (- (Transformation|GetWorldLocation (Variables|Default|GetCameraBoom)) _returnvalue))) (* (Variables|SlideToCursor|GetClampedCameraHeight) (Variables|SlideToCursor|GetfMaxClampDistanceLogicMouseCursorStart))))
          (Transformation|SetWorldLocation _cameraboom_2 (Math|Vector|MakeVector (+ (.X (Math|Vector2D|BreakVector2D (* (Math|Vector2D|Normalize2D (Math|Conversions|ToVector2D(Vector) (Math|Vector|GetForwardVector (Math|Rotator|FindLookatRotation _returnvalue (Transformation|GetWorldLocation _returnvalue_3))))) (Variables|SlideToCursor|GetfSpeedChangeLocationCameraToCursor)))) (.x _returnvalue_2)) (+ (.Y (Math|Vector2D|BreakVector2D (* (Math|Vector2D|Normalize2D (Math|Conversions|ToVector2D(Vector) (Math|Vector|GetForwardVector (Math|Rotator|FindLookatRotation _returnvalue (Transformation|GetWorldLocation _returnvalue_3))))) (Variables|SlideToCursor|GetfSpeedChangeLocationCameraToCursor)))) (.y _returnvalue_2)) (.z _returnvalue_2)) false false))
        (else
          (Transformation|SetWorldLocation _cameraboom (Math|Interpolation|VInterpTo (Transformation|GetWorldLocation _cameraboom) (Transformation|GetWorldLocation (Variables|Default|GetCapsuleComponent)) NewParam (Variables|SlideToCursor|GetfSpeedReturnCameraDeltaPosition)) false false :!label _label)))
      (else
        (goto _label)))
    (else
      (goto _label))))

(fn DropItem
  (params (DropItemInfo :type Drop%20Item%20Structure))
  (Game|SpawnActorfromClass "/Game/Blueprint/InteractEnvir/PickUpActor_Weapon.PickUpActor_Weapon_C" (Math|Transform|MakeTransform (+ (Transformation|GetActorLocation) (* (Transformation|GetActorForwardVector) 5.0))) "AlwaysSpawn" 0 DropItemInfo 0))

(fn TryPickUpActorPressed
  (bind _interactpickupactor (Variables|Default|GetInteractPickUpActor))
  (bind _overlappingactors (Collision|GetOverlappingActors _interactpickupactor "/Game/Blueprint/InteractEnvir/PickUpActor_Weapon.PickUpActor_Weapon_C" :!class /Script/Engine.PrimitiveComponent))
  (bind _output (Utilities|Array|Get(acopy) _overlappingactors))
  (Utilities|IsValid _output
    (:Is%20Valid
      (bind _aspick_up_actor_weapon (Utilities|Casting|CastToPickUpActor_Weapon _output))
      (bind _returnvalue (Class|CharacterInventoryComponent|TryGetWeapontoInventory (Variables|Default|GetCharacterInventoryComponent) (.WeaponInfo (Utilities|Struct|BreakDropItem (Variables|/Game/Blueprint/InteractEnvir/PickUpActor_Weapon.PickUpActor_Weapon_C|GetWeaponInfoDrop _aspick_up_actor_weapon)))))
      (if _returnvalue
        (Audio|PlaySound2D "/Game/Items/GameActor/Weapons/Sound/Rifle/Rifle_Raise_Cue.Rifle_Raise_Cue" 1.0 1.0 0.0 0 0)
        (Audio|PushSoundMixModifier "/Game/Sounds/MIX_Main.MIX_Main")
        (Default|PickUpSuccess _aspick_up_actor_weapon)))))